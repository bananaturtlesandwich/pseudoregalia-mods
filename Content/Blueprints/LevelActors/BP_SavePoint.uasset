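; BP_SavePoint is a level actor that wraps an ORIG_SavePoint, adding conditional player healing.
; On BeginPlay it spawns that actor at its own transform, copies its active state and player start, then binds to its box overlap after a short delay.
; When player zero enters without having ObtainedAttack, it activates the save and heals them.
; SetActive and ActivateSave forward to the spawned save point.
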(event Custom|enter
  (params (OverlappedComponent :type Primitive%20Component%20Object%20Reference) (OtherActor :type Actor%20Object%20Reference) (OtherComp :type Primitive%20Component%20Object%20Reference) (OtherBodyIndex :type Integer) (bFromSweep :type Boolean) (SweepResult :type Hit%20Result%20Structure%20%28by%20ref%29))
  (bind _returnvalue (Game|GetPlayerCharacter 0))
  (if (== _returnvalue OtherActor)
    (bind _asbp_player_goat_main (Utilities|Casting|CastToBP_PlayerGoatMain _returnvalue))
    (if (not (Variables|/Game/ThirdPerson/Player/BP_PlayerGoatMain.BP_PlayerGoatMain_C|GetobtainedAttack? _asbp_player_goat_main))
      (Default|ActivateSave (Variables|Default|Getsave%20point))
      (Default|HealPlayer _asbp_player_goat_main 1e+03))))

(event EventBeginPlay
  (bind _returnvalue (Game|SpawnActorfromClass "/Game/Blueprints/LevelActors/ORIG_SavePoint.ORIG_SavePoint_C" (Transformation|GetActorTransform) "Undefined" 0 0))
  (bind _output_get (Variables|Default|Setsave%20point _returnvalue))
  (Variables|/Game/Blueprints/LevelActors/ORIG_SavePoint.ORIG_SavePoint_C|Setactive? _output_get (Variables|Default|Getactive?))
  (Variables|/Game/Blueprints/LevelActors/ORIG_SavePoint.ORIG_SavePoint_C|SetassociatedPlayerStart _output_get (Variables|Default|GetassociatedPlayerStart))
  (Utilities|FlowControl|Delay 1.0)
  (Collision|BindEventtoOnComponentBeginOverlap (Variables|/Game/Blueprints/LevelActors/ORIG_SavePoint.ORIG_SavePoint_C|GetBox _output_get) (delegate Custom|enter)))

(fn ConstructionScript)

(fn SetActive
  (params (Condition :type Boolean))
  (Default|SetActive (Variables|Default|Getsave%20point) Condition))

(fn ActivateSave
  (Default|ActivateSave (Variables|Default|Getsave%20point)))