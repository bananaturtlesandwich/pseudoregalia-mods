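; Base upgrade pickup that grants a skill to the player on overlap, saves its collected state and destroys itself.
; A Hook added to the vanilla logic first makes slide/SlideJump and powerBoost/projectile progressive, swapping RowName and DT_UpgradeData row by player abilities.
; GameInstance receives the skill, then tier 0 opens a paused full prompt and stops music, while other tiers or debug show a mini popup.
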(event OnComponentBeginOverlap(Sphere)
  (params (OverlappedComponent :type Primitive%20Component%20Object%20Reference) (OtherActor :type Actor%20Object%20Reference) (OtherComp :type Primitive%20Component%20Object%20Reference) (OtherBodyIndex :type Integer) (bFromSweep :type Boolean) (SweepResult :type Hit%20Result%20Structure%20%28by%20ref%29))
  (bind _returnvalue (Game|GetPlayerController 0))
  (bind _returnvalue_2 (Transformation|GetActorLocation))
  (bind _upgradedata (Variables|Default|GetupgradeData))
  ;[1 0.7721 0.1287 1 50] vanilla stuff
  (CallFunction|Hook)
  (if (== (Game|GetPlayerCharacter 0) OtherActor)
    (bind _asmv_game_instance (Utilities|Casting|CastToMV_GameInstance (Game|GetGameInstance)))
    (Default|GetNewUpgradeSkill _asmv_game_instance (Variables|Default|GetrowName))
    (Default|UpdateActorSaveData (Variables|Default|GetsaveComponent))
    (Niagara|SpawnSystematLocation 0 (Transformation|GetActorLocation))
    (if (or (!= (.poweruptier (Variables|Default|GetupgradeData)) 0) (Variables|Default|GetdebugQuickPickup))
      (bind _returnvalue_3 (UserInterface|CreateWidget "/Game/UI/UI_MiniPopup.UI_MiniPopup_C" _returnvalue))
      (UserInterface|Viewport|AddtoViewport _returnvalue_3 0)
      (Default|SetInfo _returnvalue_3 "Gained an aspect of" (.displayname _upgradedata) (.instructions _upgradedata))
      (Niagara|SpawnSystematLocation 0 _returnvalue_2)
      (Audio|SpawnSoundatLocation "/Game/Audio/Sounds/cue_keyGet.cue_keyGet" _returnvalue_2 "0, 0, 0" 1.0 1.0 0.0 0 0)
      (Niagara|SpawnSystematLocation "/Game/VFX/NS_PickupSmallPowerup.NS_PickupSmallPowerup" (Transformation|GetWorldLocation (Variables|Default|GetSphere)))
      (else
        (Audio|SpawnSound2D "/Game/Audio/Sounds/cue_UpgradeGet.cue_UpgradeGet" 0.35 1.0 0.0 0)
        (bind _returnvalue_4 (UserInterface|CreateWidget "/Game/UI/UI_NewUpgradePrompt.UI_NewUpgradePrompt_C" _returnvalue))
        (Default|SetInfo _returnvalue_4 (.displayname _upgradedata) (.instructions _upgradedata) (.description _upgradedata) (.displayimage _upgradedata))
        (Input|SetInputModeUIOnly _returnvalue _returnvalue_4 "DoNotLock" false)
        (Game|SetGamePaused true)
        (UserInterface|Viewport|AddtoViewport _returnvalue_4 0)
        (bind _returnvalue_5 (Actor|GetActorOfClass "/Game/Blueprints/BP_MusicManager.BP_MusicManager_C"))
        (Utilities|IsValid _returnvalue_5
          (:Is%20Valid
            (Default|StopandSave _returnvalue_5))
          (:Is%20Not%20Valid
            _))))
    (Actor|DestroyActor)))

(event EventBPIonSuccesfulLoad
  (params (actorState :type Integer))
  (if (== actorState 1)
    (Actor|DestroyActor)))

(fn ConstructionScript
  (Rendering|Components|TextRender|SetText (Variables|Default|GetTextRender) (Utilities|Text|ToText(Name) (Variables|Default|GetrowName)))
  (if (== (.poweruptier (Variables|Default|GetupgradeData)) 0)
    (Class|NiagaraComponent|SetAsset (Variables|Default|GetNiagara) "/Game/VFX/Systems/NS_SmallUpgradeAura.NS_SmallUpgradeAura" true)))

(fn Hook
  (bind _asbp_player_goat_main (Utilities|Casting|CastToBP_PlayerGoatMain (Game|GetPlayerCharacter 0)))
  (if (and (== (Variables|Default|GetrowName) "SlideJump") (not (Variables|/Game/ThirdPerson/Player/BP_PlayerGoatMain.BP_PlayerGoatMain_C|GetobtainedSlide? _asbp_player_goat_main)))
    (bind _output_get (Variables|Default|SetrowName "slide"))
    (bind _returnvalue (Utilities|GetDataTableRow "/Game/Data/Datatables/DT_UpgradeData.DT_UpgradeData" _output_get)
      (:then
        (Variables|Default|SetupgradeData _returnvalue)))
    (elif (and (== (Variables|Default|GetrowName) "projectile") (not (Variables|/Game/ThirdPerson/Player/BP_PlayerGoatMain.BP_PlayerGoatMain_C|GetobtainedChargeAttack? _asbp_player_goat_main)))
      (bind _output_get_2 (Variables|Default|SetrowName "powerBoost"))
      (bind _returnvalue_2 (Utilities|GetDataTableRow "/Game/Data/Datatables/DT_UpgradeData.DT_UpgradeData" _output_get_2)
        (:then
          (Variables|Default|SetupgradeData _returnvalue_2)))
      (elif (and (== (Variables|Default|GetrowName) "slide") (Variables|/Game/ThirdPerson/Player/BP_PlayerGoatMain.BP_PlayerGoatMain_C|GetobtainedSlide? _asbp_player_goat_main))
        (bind _output_get_3 (Variables|Default|SetrowName "SlideJump"))
        (bind _returnvalue_3 (Utilities|GetDataTableRow "/Game/Data/Datatables/DT_UpgradeData.DT_UpgradeData" _output_get_3)
          (:then
            (Variables|Default|SetupgradeData _returnvalue_3)))
        (elif (and (== (Variables|Default|GetrowName) "powerBoost") (Variables|/Game/ThirdPerson/Player/BP_PlayerGoatMain.BP_PlayerGoatMain_C|GetobtainedChargeAttack? _asbp_player_goat_main))
          (bind _output_get_4 (Variables|Default|SetrowName "projectile"))
          (bind _returnvalue_4 (Utilities|GetDataTableRow "/Game/Data/Datatables/DT_UpgradeData.DT_UpgradeData" _output_get_4)
            (:then
              (Variables|Default|SetupgradeData _returnvalue_4))))))))