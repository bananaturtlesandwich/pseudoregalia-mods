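; SplitCling is an upgrade pickup, apparently modded from the vanilla one, that grants its RowName skill when the player overlaps it.
; It saves its collected state, shows a mini popup or paused full prompt by tier, then destroys itself.
; The added Hook handles "wallRide": using ownership captured before granting, it sets or raises the wall-run cling limit in a per-slot "Cling Gem" save and copies it to the player.
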(event OnComponentBeginOverlap(Sphere)
  (params (OverlappedComponent :type Primitive%20Component%20Object%20Reference) (OtherActor :type Actor%20Object%20Reference) (OtherComp :type Primitive%20Component%20Object%20Reference) (OtherBodyIndex :type Integer) (bFromSweep :type Boolean) (SweepResult :type Hit%20Result%20Structure%20%28by%20ref%29))
  (bind _returnvalue (Game|GetPlayerController 0))
  (bind _returnvalue_2 (Transformation|GetActorLocation))
  (bind _returnvalue_3 (Game|GetPlayerCharacter 0))
  (bind _upgradedata (Variables|Default|GetupgradeData))
  ;[1 0.7721 0.1287 1 50] vanilla stuff
  (if (== _returnvalue_3 OtherActor)
    (bind _asbp_player_goat_main (Utilities|Casting|CastToBP_PlayerGoatMain _returnvalue_3))
    (Variables|Default|Setobtained%20cling (Variables|/Game/ThirdPerson/Player/BP_PlayerGoatMain.BP_PlayerGoatMain_C|GetobtainedWallRide? _asbp_player_goat_main))
    (bind _asmv_game_instance (Utilities|Casting|CastToMV_GameInstance (Game|GetGameInstance)))
    (Default|GetNewUpgradeSkill _asmv_game_instance (Variables|Default|GetrowName))
    (Default|UpdateActorSaveData (Variables|Default|GetsaveComponent) 1 0.0)
    (Niagara|SpawnSystematLocation 0 (Transformation|GetActorLocation))
    (if (or (!= (.poweruptier (Variables|Default|GetupgradeData)) 0) (Variables|Default|GetdebugQuickPickup))
      (bind _returnvalue_4 (UserInterface|CreateWidget "/Game/UI/UI_MiniPopup.UI_MiniPopup_C" _returnvalue))
      (UserInterface|Viewport|AddtoViewport _returnvalue_4 0)
      (Default|SetInfo _returnvalue_4 "Gained an aspect of" (.displayname _upgradedata) (.instructions _upgradedata))
      (Niagara|SpawnSystematLocation 0 _returnvalue_2)
      (Audio|SpawnSoundatLocation "/Game/Audio/Sounds/cue_keyGet.cue_keyGet" _returnvalue_2 "0, 0, 0" 1.0 1.0 0.0 0 0)
      (Niagara|SpawnSystematLocation "/Game/VFX/NS_PickupSmallPowerup.NS_PickupSmallPowerup" (Transformation|GetWorldLocation (Variables|Default|GetSphere)))
      (else
        (Audio|SpawnSound2D "/Game/Audio/Sounds/cue_UpgradeGet.cue_UpgradeGet" 0.35 1.0 0.0 0)
        (bind _returnvalue_5 (UserInterface|CreateWidget "/Game/UI/UI_NewUpgradePrompt.UI_NewUpgradePrompt_C" _returnvalue))
        (Default|SetInfo _returnvalue_5 (.displayname _upgradedata) (.instructions _upgradedata) (.description _upgradedata) (.displayimage _upgradedata))
        (Input|SetInputModeUIOnly _returnvalue _returnvalue_5 "DoNotLock" false)
        (Game|SetGamePaused true)
        (UserInterface|Viewport|AddtoViewport _returnvalue_5 0)
        (bind _returnvalue_6 (Actor|GetActorOfClass "/Game/Blueprints/BP_MusicManager.BP_MusicManager_C"))
        (Utilities|IsValid _returnvalue_6
          (:Is%20Valid
            (Default|StopandSave _returnvalue_6))
          (:Is%20Not%20Valid
            _))))
    (CallFunction|Hook)
    (Actor|DestroyActor)))

(event EventBPIonSuccesfulLoad
  (params (actorState :type Integer))
  (if (== actorState 1)
    (Actor|DestroyActor)))

(fn ConstructionScript
  (Rendering|Components|TextRender|SetText (Variables|Default|GetTextRender) (Utilities|Text|ToText(Name) (Variables|Default|GetrowName))))

(fn Hook
  (if (== (Variables|Default|GetrowName) "wallRide")
    (bind _asmv_game_instance (Utilities|Casting|CastToMV_GameInstance (Game|GetGameInstance)))
    (bind _returnvalue (SaveGame|LoadGamefromSlot (Utilities|String|Append "Cling Gem " (Variables|/Game/Blueprints/GameData/MV_GameInstance.MV_GameInstance_C|GetactiveSaveSlotName _asmv_game_instance))))
    (bind _aswall_run_cling_limit (Utilities|Casting|CastToWallRunClingLimit _returnvalue)
      (:then
        (bind _output_get (LocalVariables|Setsave _aswall_run_cling_limit))
        (if (Variables|Default|Getobtained%20cling)
          (bind _output_get_2 (Variables|/Game/Blueprints/WallRunClingLimit.WallRunClingLimit_C|SetwallRunClingLimit _output_get (+ (stale _output_get_2) 2)))
          (else
            (Variables|/Game/Blueprints/WallRunClingLimit.WallRunClingLimit_C|SetwallRunClingLimit _output_get 1))))
      (:CastFailed
        (bind _returnvalue_2 (SaveGame|CreateSaveGameObject "/Game/Blueprints/WallRunClingLimit.WallRunClingLimit_C"))
        (bind _output_get_3 (LocalVariables|Setsave _returnvalue_2))))
    (SaveGame|SaveGametoSlot _output_get_3 (Utilities|String|Append "Cling Gem " (Variables|/Game/Blueprints/GameData/MV_GameInstance.MV_GameInstance_C|GetactiveSaveSlotName _asmv_game_instance)))
    (bind _asbp_player_goat_main (Utilities|Casting|CastToBP_PlayerGoatMain (Game|GetPlayerCharacter 0)))
    (Variables|/Game/ThirdPerson/Player/BP_PlayerGoatMain.BP_PlayerGoatMain_C|SetwallRunClingLimit _asbp_player_goat_main (Variables|/Game/Blueprints/WallRunClingLimit.WallRunClingLimit_C|GetwallRunClingLimit (LocalVariables|Getsave)))))