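; BP_UpgradeBase places an upgrade in the world, matching it to the player goat's progress.
; On BeginPlay it spawns an ORIG_UpgradeBase and an overlap trigger, then destroys stray upgrade instances at the world origin.
; Player overlap swaps slide/SlideJump or powerBoost/projectile based on obtained abilities, reloading DT_UpgradeData and passing it to the spawned upgrade.
; Destruction of that upgrade saves state through SaveComponent, so loading removes already-taken upgrades.
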(event Custom|save
  (params (DestroyedActor :type Actor%20Object%20Reference))
  (Default|UpdateActorSaveData (Variables|Default|GetsaveComponent) 1)
  (Actor|DestroyActor (stale EventBeginPlay _returnvalue_2))
  (Actor|DestroyActor))

(event Custom|tweak
  (params (OverlappedActor :type Actor%20Object%20Reference) (OtherActor :type Actor%20Object%20Reference))
  (bind _returnvalue (Game|GetPlayerCharacter 0))
  (if (== _returnvalue OtherActor)
    (bind _asbp_player_goat_main (Utilities|Casting|CastToBP_PlayerGoatMain _returnvalue))
    (if (and (== (Variables|Default|GetrowName) "SlideJump") (not (Variables|/Game/ThirdPerson/Player/BP_PlayerGoatMain.BP_PlayerGoatMain_C|GetobtainedSlide? _asbp_player_goat_main)))
      (bind _output_get (Variables|Default|SetrowName "slide"))
      (bind _returnvalue_2 (Utilities|GetDataTableRow "/Game/Data/Datatables/DT_UpgradeData.DT_UpgradeData" _output_get)
        (:then
          (Variables|Default|SetupgradeData _returnvalue_2)
          (CallFunction|Finalise (stale EventBeginPlay _returnvalue_3) :!label _label)))
      (elif (and (== (Variables|Default|GetrowName) "projectile") (not (Variables|/Game/ThirdPerson/Player/BP_PlayerGoatMain.BP_PlayerGoatMain_C|GetobtainedChargeAttack? _asbp_player_goat_main)))
        (bind _output_get_2 (Variables|Default|SetrowName "powerBoost"))
        (bind _returnvalue_3 (Utilities|GetDataTableRow "/Game/Data/Datatables/DT_UpgradeData.DT_UpgradeData" _output_get_2)
          (:then
            (Variables|Default|SetupgradeData _returnvalue_3)
            (CallFunction|Finalise (stale EventBeginPlay _returnvalue_3))))
        (elif (and (== (Variables|Default|GetrowName) "slide") (Variables|/Game/ThirdPerson/Player/BP_PlayerGoatMain.BP_PlayerGoatMain_C|GetobtainedSlide? _asbp_player_goat_main))
          (bind _output_get_3 (Variables|Default|SetrowName "SlideJump"))
          (bind _returnvalue_4 (Utilities|GetDataTableRow "/Game/Data/Datatables/DT_UpgradeData.DT_UpgradeData" _output_get_3)
            (:then
              (Variables|Default|SetupgradeData _returnvalue_4)
              (CallFunction|Finalise (stale EventBeginPlay _returnvalue_3))))
          (elif (and (== (Variables|Default|GetrowName) "powerBoost") (Variables|/Game/ThirdPerson/Player/BP_PlayerGoatMain.BP_PlayerGoatMain_C|GetobtainedChargeAttack? _asbp_player_goat_main))
            (bind _output_get_4 (Variables|Default|SetrowName "projectile"))
            (bind _returnvalue_5 (Utilities|GetDataTableRow "/Game/Data/Datatables/DT_UpgradeData.DT_UpgradeData" _output_get_4)
              (:then
                (Variables|Default|SetupgradeData _returnvalue_5)
                (CallFunction|Finalise (stale EventBeginPlay _returnvalue_3))))
            (else
              (goto _label))))))
    (else
      (CallFunction|Finalise (stale EventBeginPlay _returnvalue_3)))))

(event EventBeginPlay
  (bind _returnvalue (Transformation|GetActorTransform))
  (bind _returnvalue_2 (Game|SpawnActorfromClass "/Script/Engine.TriggerSphere" (Math|Transform|MakeTransform (+ (.location _returnvalue) "0.000000,0.000000,100.000000") (.rotation _returnvalue) "5.000000,5.000000,5.000000") "Undefined" 0 0))
  (Collision|BindEventtoOnActorBeginOverlap _returnvalue_2 (delegate Custom|tweak))
  (bind _returnvalue_3 (Game|SpawnActorfromClass "/Game/Blueprints/ORIG_UpgradeBase.ORIG_UpgradeBase_C" (Transformation|GetActorTransform) "Undefined" 0 0))
  (Game|BindEventtoOnDestroyed _returnvalue_3 (delegate Custom|save) :!label _label)
  (bind _outactors (Actor|GetAllActorsOfClass "/Game/Blueprints/ORIG_UpgradeBase.ORIG_UpgradeBase_C"))
  (for _array_element _outactors
    (if (Utilities|Operators|EqualEqual :A (Transformation|GetActorLocation _array_element))
      (Actor|DestroyActor _array_element)
      (goto _label))))

(event EventBPIonSuccesfulLoad
  (params (actorState :type Integer))
  (if (== actorState 1)
    (Actor|DestroyActor (stale EventBeginPlay _returnvalue_2))
    (Actor|DestroyActor (stale EventBeginPlay _returnvalue_3))
    (Actor|DestroyActor)))

(fn ConstructionScript)

(fn Finalise
  (params (upgrade :type ORIG%20Upgrade%20Base%20Object%20Reference))
  (Variables|/Game/Blueprints/ORIG_UpgradeBase.ORIG_UpgradeBase_C|SetrowName upgrade (Variables|Default|GetrowName))
  (Variables|/Game/Blueprints/ORIG_UpgradeBase.ORIG_UpgradeBase_C|SetupgradeData upgrade (Variables|Default|GetupgradeData)))

(fn Debug
  (params (text :type Text))
  (bind _returnvalue (UserInterface|CreateWidget "/Game/UI/UI_MiniPopup.UI_MiniPopup_C" (Game|GetPlayerController 0)))
  (UserInterface|Viewport|AddtoViewport _returnvalue 0)
  (Default|SetInfo _returnvalue text))